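; BP_Crystal is a pickup-style crystal that flies into the player pawn and vanishes, without granting anything itself.
; On overlap it disables its sphere trigger and caches its location, scale and light intensity.
; A timeline lerps it to the pawn's live position while shrinking it and fading its point light, then destroys it.
; The IsPlayer check receives the player pawn instead of the overlapping actor, so any overlap passes.
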(event `self.ReceiveActorBeginOverlap`
  (params (OtherActor :type "Actor Object Reference"))
  (`self.IsPlayer` (`GameplayStatics.GetPlayerPawn` 0)
    (:`IsPlayer`
      (`PrimitiveComponent.SetCollisionEnabled` (`self.SphereTrigger`) "NoCollision")
      (`self.CrystalPosition`)
      (`self.CrystalScale`)
      (`self.Lerp Intensity`)
      (bind (_direction _smoothlerpalpha _scale _intensity) (`Timeline|TL_BlendAlpha`)
        (:`Update`
          (`self.CrystalToPawn` _smoothlerpalpha)
          (`self.Scale` _scale)
          (`self.Intensity` _intensity))
        (:`Finished`
          (`self.K2_DestroyActor`))))))

(fn `CrystalPosition`
  (set `self.LerpStartLocation` (`self.K2_GetActorLocation`)))

(fn `CrystalScale`
  (set `self.LerpStartScale` (`self.GetActorScale3D`)))

(fn `CrystalToPawn`
  (params (Alpha :type "Float (double-precision)"))
  (`self.K2_SetActorLocation` (`KismetMathLibrary.VLerp` (`self.LerpStartLocation`) (`self.K2_GetActorLocation` (`GameplayStatics.GetPlayerPawn` 0)) Alpha)))

(fn `Intensity`
  (params (Alpha :type "Float (double-precision)"))
  (`LightComponent.SetIntensity` (`self.PointLight`) (`KismetMathLibrary.Lerp` (`self.Intensitylerp`) 0.0 Alpha)))

(fn `Lerp Intensity`
  (set `self.Intensitylerp` (`LightComponentBase.Intensity` (`self.PointLight`))))

(fn `Scale`
  (params (Alpha :type "Float (double-precision)"))
  (`self.SetActorScale3D` (`KismetMathLibrary.VLerp` (`self.LerpStartScale`) (0.0 0.0 0.0) Alpha)))

(fn `UserConstructionScript`)